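; NPC Blueprint that displays its 3D mesh as a real-time rendered, camera-facing sprite.
; BeginPlay hides the mesh from everything but scene captures, limits the capture to this actor and feeds its render target into a dynamic material on the sprite.
; Each Tick moves the capture to the player camera's position aimed at the mesh.
; It also places the sprite slightly in front of the mesh, oriented by camera look-at plus fixed offsets.
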(event EventBeginPlay
  (bind _returnvalue (CanvasRenderTarget2D|CreateCanvasRenderTarget2D "/Script/Engine.CanvasRenderTarget2D" 1024 1024))
  (bind _output_get (Variables|/Script/Engine.SceneCaptureComponent2D|SetTextureTarget (Variables|Default|GetSceneCaptureComponent2D) _returnvalue))
  (bind _returnvalue_2 (Rendering|Material|CreateDynamicMaterialInstance "/Game/RealTimeSprites/Materials/SpriteMat.SpriteMat" "None" "None" :!class /Script/Engine.KismetMaterialLibrary))
  (Rendering|Material|SetTextureParameterValue _returnvalue_2 "Sprite" _output_get)
  (Rendering|Material|SetMaterial (Variables|Default|GetSprite) 0 _returnvalue_2)
  (Variables|/Script/Engine.SceneCaptureComponent|SetShowOnlyActors (Variables|Default|GetSceneCaptureComponent2D) (Utilities|Array|MakeArray (Components|GetOwner (Variables|Character|GetMesh))))
  (Class|PrimitiveComponent|SetVisibleinSceneCaptureOnly (Variables|Character|GetMesh) true))

(event EventTick
  (params (DeltaSeconds :type Float%20%28single-precision%29))
  (bind _returnvalue (Game|GetPlayerCameraManager 0))
  (bind _scenecapturecomponent2d (Variables|Default|GetSceneCaptureComponent2D))
  (bind _mesh (Variables|Character|GetMesh))
  (bind _sprite (Variables|Default|GetSprite))
  (bind _returnvalue_2 (Camera|GetCameraLocation _returnvalue))
  (bind _returnvalue_3 (Transformation|GetWorldLocation _sprite))
  (bind _returnvalue_4 (Math|Rotator|FindLookatRotation _returnvalue_2 _returnvalue_3))
  (bind (_roll _pitch _yaw) (Math|Rotator|BreakRotator _returnvalue_4))
  (Transformation|SetWorldLocationAndRotation _scenecapturecomponent2d (Transformation|GetWorldLocation (Variables|/Script/Engine.Actor|GetRootComponent _returnvalue)) (Math|Rotator|FindLookatRotation (Transformation|GetWorldLocation _scenecapturecomponent2d) (Transformation|GetWorldLocation _mesh)) false false)
  (Transformation|SetWorldLocationAndRotation (Variables|Default|GetSprite) (+ (Transformation|GetWorldLocation _mesh) (* (Math|Rotator|GetRotationXVector _returnvalue_4) (Math|Conversions|ToVector(Float) -1e+02))) (Math|Rotator|MakeRotator (+ _roll 45.0) (+ _pitch 45.0) (+ _yaw 9e+01)) false false))

(event Collision|EventActorBeginOverlap
  (params (OtherActor :type Actor%20Object%20Reference)))

(fn ConstructionScript)