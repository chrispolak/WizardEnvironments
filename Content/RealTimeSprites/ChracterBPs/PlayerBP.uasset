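; PlayerBP is a player Blueprint that displays its 3D mesh as a real-time sprite by rendering it to a texture.
; On BeginPlay, a scene capture limited to its own actor feeds a 1024 render target into a dynamic sprite material, and the mesh becomes visible only in scene captures.
; Each tick moves the sprite and capture component from the mesh toward the camera along its view axis, aiming the capture at the mesh.
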(event EventBeginPlay
  (bind _mesh (Variables|Character|GetMesh))
  (bind _returnvalue (CanvasRenderTarget2D|CreateCanvasRenderTarget2D "/Script/Engine.CanvasRenderTarget2D" 1024 1024))
  (Variables|/Script/Engine.SceneCaptureComponent2D|SetTextureTarget (Variables|Default|GetSceneCaptureComponent2D) _returnvalue)
  (bind _returnvalue_2 (Rendering|Material|CreateDynamicMaterialInstance "/Game/RealTimeSprites/Materials/SpriteMat.SpriteMat" "None" "None" :!class /Script/Engine.KismetMaterialLibrary))
  (Rendering|Material|SetTextureParameterValue _returnvalue_2 "Sprite" _returnvalue)
  (Rendering|Material|SetMaterial (Variables|Default|GetSprite) 0 _returnvalue_2)
  (Variables|/Script/Engine.SceneCaptureComponent|SetShowOnlyActors (Variables|Default|GetSceneCaptureComponent2D) (Utilities|Array|MakeArray (Components|GetOwner _mesh)))
  (Class|PrimitiveComponent|SetVisibleinSceneCaptureOnly _mesh true))

(event EventTick
  (params (DeltaSeconds :type Float%20%28single-precision%29))
  (bind _returnvalue (Game|GetPlayerCameraManager 0))
  (bind _mesh (Variables|Character|GetMesh))
  (bind _scenecapturecomponent2d (Variables|Default|GetSceneCaptureComponent2D))
  (bind _returnvalue_2 (Transformation|GetWorldLocation _mesh))
  (bind _transformcomponent (Variables|/Script/Engine.PlayerCameraManager|GetTransformComponent _returnvalue))
  (bind _returnvalue_3 (Math|Vector|GetForwardVector _transformcomponent))
  (Transformation|SetWorldLocation (Variables|Default|GetSprite) (+ _returnvalue_2 (* _returnvalue_3 (Math|Conversions|ToVector(Float) -2e+02))) false false)
  (Transformation|SetWorldLocation (Variables|Default|GetSceneCaptureComponent2D) (- (+ _returnvalue_2 (* _returnvalue_3 (Math|Conversions|ToVector(Float) -1e+03))) "") false false)
  (Transformation|SetWorldRotation _scenecapturecomponent2d (Math|Rotator|FindLookatRotation (Transformation|GetWorldLocation _scenecapturecomponent2d) (Transformation|GetWorldLocation _mesh)) false false))

(fn ConstructionScript)