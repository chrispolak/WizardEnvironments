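; Tree actor that acts as a billboard, turning its Tree component toward the player's camera every frame.
; Tick computes a look-at rotation from the tree to player 0's camera manager and applies its yaw and roll as world rotation, with pitch held at a fixed tilt.
; The construction script and other events are empty.
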(event EventBeginPlay)

(event Collision|EventActorBeginOverlap
  (params (OtherActor :type Actor%20Object%20Reference)))

(event EventTick
  (params (DeltaSeconds :type Float%20%28single-precision%29))
  (bind _returnvalue (Game|GetPlayerCameraManager 0))
  (bind _tree (Variables|Default|GetTree))
  (bind _returnvalue_2 (Transformation|GetWorldLocation _tree))
  (bind _rootcomponent (Variables|/Script/Engine.Actor|GetRootComponent _returnvalue))
  (bind _returnvalue_3 (Transformation|GetWorldLocation _rootcomponent))
  (bind _returnvalue_4 (Math|Rotator|FindLookatRotation _returnvalue_2 _returnvalue_3))
  (bind (_roll _pitch _yaw) (Math|Rotator|BreakRotator _returnvalue_4))
  (Transformation|SetWorldRotation (Variables|Default|GetTree) (Math|Rotator|MakeRotator _roll 2e+01 _yaw) false false))

(fn ConstructionScript)